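; Day/night controller Blueprint that switches the stars on the level's sky sphere between night and day.
; On BeginPlay it casts the assigned sky sphere actor to BP_Sky_Sphere, caches it and runs UpdateSkyState.
; UpdateSkyState sets star brightness from the IsNight flag, refreshes the sky material and prints the current state.
; Nothing in the graph changes IsNight or updates the sky after startup.
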(event EventBeginPlay
  (bind _asbp_sky_sphere (Utilities|Casting|CastToBP_Sky_Sphere (Variables|Default|GetSkySphereActor)))
  (Variables|Default|SetSkySphereRef _asbp_sky_sphere)
  (CallFunction|UpdateSkyState))

(event Collision|EventActorBeginOverlap
  (params (OtherActor :type Actor%20Object%20Reference)))

(event EventTick
  (params (DeltaSeconds :type Float%20%28single-precision%29)))

(fn ConstructionScript)

(fn UpdateSkyState
  (bind _bisnight (Variables|Default|GetbIsNight))
  (bind _skysphereref (Variables|Default|GetSkySphereRef))
  (Utilities|IsValid _skysphereref
    (:Is%20Valid
      (Variables|/Engine/EngineSky/BP_Sky_Sphere.BP_Sky_Sphere_C|SetStars%20brightness _skysphereref (Math|Float|SelectFloat 1.0 0.0 _bisnight))
      (Default|RefreshMaterial _skysphereref)
      (Development|PrintString (Utilities|String|SelectString "Night" "Day" _bisnight)))))