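; BP_DayNightController is a debug-style toggle that switches the level between day and night on BeginPlay and on each T press.
; It instantly sets post-process exposure, sun rotation and intensity, skylight intensity, height fog visibility and sky sphere stars, then refreshes the sky material.
; IsNight holds the next state to apply rather than the current one, so its default decides the starting look.
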(event EventBeginPlay
  (bind _ahfog (Variables|Default|GetAHFog))
  (bind _skysphere (Variables|Default|GetSkySphere))
  (bind _sunlight (Variables|Default|GetSunLight))
  (bind _ppv (Variables|Default|GetPPV))
  (bind _skylight (Variables|Default|GetSkyLight))
  (bind _component (Variables|/Script/Engine.ExponentialHeightFog|GetComponent _ahfog))
  (bind _settings (Variables|/Script/Engine.PostProcessVolume|GetSettings _ppv))
  (bind _lightcomponent (Variables|/Script/Engine.Light|GetLightComponent _sunlight))
  (bind _lightcomponent_2 (Variables|/Script/Engine.SkyLight|GetLightComponent _skylight))
  (if (Variables|Default|GetbIsNight)
    ;[1 1 1] Night
    (Variables|Default|SetbIsNight false)
    (Utilities|Struct|SetmembersinPostProcessSettings _settings -1.0)
    (Transformation|SetActorRotation _sunlight "90.000000, 0, 0")
    (Rendering|Components|Light|SetIntensity _lightcomponent 0.0)
    (Rendering|Components|Light|SetIntensity _lightcomponent_2 0.0)
    (Rendering|SetVisibility _component false false)
    (Variables|/Engine/EngineSky/BP_Sky_Sphere.BP_Sky_Sphere_C|SetStars%20brightness _skysphere 0.5)
    (Development|PrintString "Night")
    (else
      ;[1 1 1] Day
      (Variables|Default|SetbIsNight true)
      (Utilities|Struct|SetmembersinPostProcessSettings _settings 1.0)
      (Transformation|SetActorRotation _sunlight "-45.000000, 0, 0")
      (Rendering|Components|Light|SetIntensity _lightcomponent 1.0)
      (Rendering|Components|Light|SetIntensity _lightcomponent_2 1.0)
      (Rendering|SetVisibility _component true false)
      (Variables|/Engine/EngineSky/BP_Sky_Sphere.BP_Sky_Sphere_C|SetStars%20brightness _skysphere 0.0)
      (Development|PrintString "Day")))
  (Default|RefreshMaterial _skysphere))

(event Input|KeyboardEvents|T
  (params (Key :type Key%20Structure :default "None"))
  (bind _ahfog (Variables|Default|GetAHFog))
  (bind _skysphere (Variables|Default|GetSkySphere))
  (bind _sunlight (Variables|Default|GetSunLight))
  (bind _ppv (Variables|Default|GetPPV))
  (bind _skylight (Variables|Default|GetSkyLight))
  (bind _component (Variables|/Script/Engine.ExponentialHeightFog|GetComponent _ahfog))
  (bind _settings (Variables|/Script/Engine.PostProcessVolume|GetSettings _ppv))
  (bind _lightcomponent (Variables|/Script/Engine.Light|GetLightComponent _sunlight))
  (bind _lightcomponent_2 (Variables|/Script/Engine.SkyLight|GetLightComponent _skylight))
  (:Pressed
    (if (Variables|Default|GetbIsNight)
      ;[1 1 1] Night
      (Variables|Default|SetbIsNight false)
      (Utilities|Struct|SetmembersinPostProcessSettings _settings -1.0)
      (Transformation|SetActorRotation _sunlight "90.000000, 0, 0")
      (Rendering|Components|Light|SetIntensity _lightcomponent 0.0)
      (Rendering|Components|Light|SetIntensity _lightcomponent_2 0.0)
      (Rendering|SetVisibility _component false false)
      (Variables|/Engine/EngineSky/BP_Sky_Sphere.BP_Sky_Sphere_C|SetStars%20brightness _skysphere 0.5)
      (Development|PrintString "Night")
      (else
        ;[1 1 1] Day
        (Variables|Default|SetbIsNight true)
        (Utilities|Struct|SetmembersinPostProcessSettings _settings 1.0)
        (Transformation|SetActorRotation _sunlight "-45.000000, 0, 0")
        (Rendering|Components|Light|SetIntensity _lightcomponent 1.0)
        (Rendering|Components|Light|SetIntensity _lightcomponent_2 1.0)
        (Rendering|SetVisibility _component true false)
        (Variables|/Engine/EngineSky/BP_Sky_Sphere.BP_Sky_Sphere_C|SetStars%20brightness _skysphere 0.0)
        (Development|PrintString "Day")))
    (Default|RefreshMaterial _skysphere)))

(fn ConstructionScript)